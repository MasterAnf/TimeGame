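; BP_TimeTravelPortal is a portal actor that teleports the first-person character to a linked portal.
; On actor overlap, Teleport checks that the actor is a FirstPersonCharacter and that PortalEnd is another BP_TimeTravelPortal.
; It moves the character to the destination's Box location, sets the player controller's control rotation to that Box's rotation, then calls StopMovement on the character.
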(event EventBeginPlay)

(event Collision|EventActorBeginOverlap
  (params (OtherActor :type Actor%20Object%20Reference))
  (CallFunction|Teleport OtherActor))

(event EventTick
  (params (DeltaSeconds :type Float%20%28single-precision%29)))

(fn ConstructionScript)

(fn Teleport
  (params (Other :type Actor%20Object%20Reference))
  ;[1 1 1] Teleport
  (if (== (Utilities|GetClass Other) "/Game/FirstPersonCPP/Blueprints/FirstPersonCharacter.FirstPersonCharacter_C")
    (if (== (Utilities|GetClass (Variables|Default|GetPortalEnd)) "BP_TimeTravelPortal_C")
      (bind _asbp_time_travel_portal (Utilities|Casting|CastToBP_TimeTravelPortal (Variables|Default|GetPortalEnd)))
      (Transformation|SetActorLocationAndRotation Other (Transformation|GetWorldLocation (Variables|BP_TimeTravelPortal_C|GetBox _asbp_time_travel_portal)) "0, 0, 0" false true)
      (Pawn|SetControlRotation (Game|GetPlayerController 0) (Transformation|GetWorldRotation (Variables|BP_TimeTravelPortal_C|GetBox _asbp_time_travel_portal)))
      (bind _asfirst_person_character (Utilities|Casting|CastToFirstPersonCharacter Other))
      (Default|StopMovement _asfirst_person_character))))