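; BP_ControlBrazier is a puzzle brazier that switches on a linked network of braziers.
; TurnOnNetwork runs only while unpowered, then marks itself and every BrazierNetwork member as powered.
; It gives them all the same fixed SelectedColor and calls SetFire on each, finishing with itself.
; The event graph holds only disabled default events, so the function relies on an external call.
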(event EventBeginPlay
  (|CallParentFunction))

(event Collision|EventActorBeginOverlap
  (params (OtherActor :type Actor%20Object%20Reference)))

(event EventTick
  (params (DeltaSeconds :type Float%20%28single-precision%29)))

(fn ConstructionScript
  (|CallParentFunction))

(fn TurnonNetwork
  (if (not (Variables|Default|GetPowered))
    (Variables|Default|SetPowered true)
    (for _array_element (Variables|Default|GetBrazierNetwork)
      (Variables|/Game/PuzzleCPP/BP_Brazier.BP_Brazier_C|SetPowered _array_element true)
      (Variables|/Game/PuzzleCPP/BP_Brazier.BP_Brazier_C|SetSelectedColor _array_element "NewEnumerator4")
      (Default|SetFire _array_element))
    (Variables|Default|SetSelectedColor "NewEnumerator4")
    (CallFunction|SetFire)))