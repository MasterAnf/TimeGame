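; BP_Brazier is a puzzle brazier whose fire color can be cycled.
; SetFire maps the SelectedColor enum to a particle template on the Fire component, using ambient dust for Off, and runs in the construction script.
; BeginPlay calls SetTemplate with no template, clearing the constructed effect.
; IncrementColor works only when Powered, advancing the enum, wrapping to Red instead of landing on Off, then refreshing the fire.
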(event EventBeginPlay
  (Effects|Components|ParticleSystem|SetTemplate (Variables|Default|GetFire) 0))

(event Collision|EventActorBeginOverlap
  (params (OtherActor :type Actor%20Object%20Reference)))

(event EventTick
  (params (DeltaSeconds :type Float%20%28single-precision%29)))

(fn ConstructionScript
  (CallFunction|SetFire))

(fn SetFire
  (switch Utilities|FlowControl|Switch|SwitchonEnum_Color (Variables|Default|GetSelectedColor)
    (:NewEnumerator0
      (Effects|Components|ParticleSystem|SetTemplate (Variables|Default|GetFire) "/Game/StarterContent/Particles/P_Fire_Red.P_Fire_Red"))
    (:NewEnumerator1
      (Effects|Components|ParticleSystem|SetTemplate (Variables|Default|GetFire) "/Game/StarterContent/Particles/P_Fire_Blue.P_Fire_Blue"))
    (:NewEnumerator2
      (Effects|Components|ParticleSystem|SetTemplate (Variables|Default|GetFire) "/Game/StarterContent/Particles/P_Fire_Green.P_Fire_Green"))
    (:NewEnumerator3
      (Effects|Components|ParticleSystem|SetTemplate (Variables|Default|GetFire) "/Game/StarterContent/Particles/P_Fire_Yellow.P_Fire_Yellow"))
    (:NewEnumerator4
      (Effects|Components|ParticleSystem|SetTemplate (Variables|Default|GetFire) "/Game/StarterContent/Particles/P_Fire_White.P_Fire_White"))
    (:NewEnumerator5
      (Effects|Components|ParticleSystem|SetTemplate (Variables|Default|GetFire) "/Game/StarterContent/Particles/P_Fire_Purple.P_Fire_Purple"))
    (:NewEnumerator6
      (Effects|Components|ParticleSystem|SetTemplate (Variables|Default|GetFire) "/Game/StarterContent/Particles/P_Ambient_Dust.P_Ambient_Dust"))))

(fn IncrementColor
  (if (Variables|Default|GetPowered)
    (bind _output_get (Variables|Default|SetSelectedColor (Utilities|Enum|ByteToEnumEnum_Color (+ (Variables|Default|GetSelectedColor) 1))))
    (if (Utilities|Enum|Equal(Enum) _output_get "NewEnumerator6")
      (Variables|Default|SetSelectedColor "NewEnumerator0"))
    (CallFunction|SetFire)))